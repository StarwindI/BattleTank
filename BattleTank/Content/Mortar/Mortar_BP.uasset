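; Mortar Blueprint that sets up a turret with aiming and a health bar display.
; On BeginPlay it passes its MortarDome and MortarBarrel to the TankAiming component as turret and barrel.
; It then casts the HealthUi widget to HealthBar_BP and sets itself as that widget's Healthy reference.
; The graphs hold only this wiring, with no firing or damage logic.
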(event EventBeginPlay
  (Class|TankAimingComponent|SetTurretBarrel (Variables|Default|GetTankAiming) (Variables|Default|Getmortar_dome) (Variables|Default|Getmortar_barrel))
  (CallFunction|SetHealthBarWidget))

(fn ConstructionScript)

(fn SetHealthBarWidget
  (bind _ashealth_bar_bp (Utilities|Casting|CastToHealthBar_BP (UserInterface|GetUserWidgetObject (Variables|Default|Gethealth_ui))))
  (Variables|/Game/UI/HealthBar_BP.HealthBar_BP_C|SetHealthy _ashealth_bar_bp self)
  (return))