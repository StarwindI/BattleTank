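; Player-controllable tank Blueprint that maps input to driving, camera orbit and zoom, and firing.
; Separate axes feed throttle to the left and right tracks for differential steering.
; Aim axes rotate an azimuth gimbal and spring arm, scaled by frame time, while zoom adjusts the clamped arm length.
; BeginPlay registers the turret and barrel through setters; setters and Fire are defined outside this graph.
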(event EventBeginPlay
  ;[1 1 1] Tank setup
  (Class|Tank|SetTurret (Variables|Default|Getturret))
  (Class|Tank|SetBarrel (Variables|Default|Getbarrel)))

(event Input|ActionEvents|InputActionFire
  (params (Key :type Key%20Structure :default "AnyKey"))
  ;[1 1 1] Tank setup
  (:Pressed
    (Class|Tank|Fire)))

(event Input|AxisEvents|InputAxisAimAzimuth
  (params (AxisValue :type Float%20%28single-precision%29))
  ;[1 1 1] Input setup
  (Transformation|AddLocalRotation (Variables|Default|GetAzimuthGimble) (Math|Rotator|MakeRotator 0.0 0.0 (* AxisValue (Utilities|Time|GetWorldDeltaSeconds) 1e+02)) false false))

(event Input|AxisEvents|InputAxisRightTrackThrottle
  (params (AxisValue :type Float%20%28single-precision%29))
  (Class|TankTrack|SetThrottle (Variables|Default|Getright_track) AxisValue))

(event Input|AxisEvents|InputAxisAimAltitude
  (params (AxisValue :type Float%20%28single-precision%29))
  ;[1 1 1] Input setup
  (Transformation|AddLocalRotation (Variables|Default|GetSpringArm) (Math|Rotator|MakeRotator 0.0 (* AxisValue (Utilities|Time|GetWorldDeltaSeconds) 1e+02) 0.0) false false))

(event Input|AxisEvents|InputAxisLeftTrackThrottle
  (params (AxisValue :type Float%20%28single-precision%29))
  (Class|TankTrack|SetThrottle (Variables|Default|Getleft_track) AxisValue))

(event Input|AxisEvents|InputAxisZoom
  (params (AxisValue :type Float%20%28single-precision%29))
  ;[1 1 1] Input setup
  (Variables|/Script/Engine.SpringArmComponent|SetTargetArmLength (Variables|Default|GetSpringArm) (Math|Float|Clamp(Float) (+ (* AxisValue 1e+02) (Variables|/Script/Engine.SpringArmComponent|GetTargetArmLength (Variables|Default|GetSpringArm))) 5e+02 1e+04)))

(fn ConstructionScript)